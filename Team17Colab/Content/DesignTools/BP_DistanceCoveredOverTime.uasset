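; Design tool that measures how long an overlapping actor takes to cover a set distance between Start and End components.
; The construction script places End along X at RelativeOffset.
; Beginning overlap with Start starts a looping timer with an empty callback, used as a stopwatch that wraps every 100 seconds.
; Ending overlap with End prints the offset and elapsed time, then clears the timer.
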(event OnComponentBeginOverlap(Start)
  (params (OverlappedComponent :type Primitive%20Component%20Object%20Reference) (OtherActor :type Actor%20Object%20Reference) (OtherComp :type Primitive%20Component%20Object%20Reference) (OtherBodyIndex :type Integer) (bFromSweep :type Boolean) (SweepResult :type Hit%20Result%20Structure%20%28by%20ref%29))
  (bind _returnvalue (Utilities|Time|SetTimerbyEvent (delegate Custom|Hello) 1e+02 true))
  (Variables|Default|SetTimer _returnvalue))

(event OnComponentEndOverlap(End)
  (params (OverlappedComponent :type Primitive%20Component%20Object%20Reference) (OtherActor :type Actor%20Object%20Reference) (OtherComp :type Primitive%20Component%20Object%20Reference) (OtherBodyIndex :type Integer))
  (Development|PrintString (Utilities|String|Append (Utilities|String|ToString(Float) (Variables|Default|GetRelativeOffset)) " distance, time: " (Utilities|String|ToString(Float) (Class|KismetSystemLibrary|GetTimerElapsedTimeHandle (Variables|Default|GetTimer)))))
  (Utilities|Time|ClearandInvalidateTimerbyHandle (Variables|Default|GetTimer)))

(event Custom|Hello)

(fn ConstructionScript
  (Transformation|SetRelativeLocation (Variables|Default|GetEnd) (Math|Vector|MakeVector (Variables|Default|GetRelativeOffset) 0.0 0.0) false false))