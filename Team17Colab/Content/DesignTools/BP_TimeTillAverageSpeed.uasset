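; Design debug actor that measures how long the PhysicsBallBP ball takes to exceed its SpeedLock speed and the distance from its start point.
; Tick polls ball velocity, using a looping timer with an empty event as a stopwatch that starts on movement and clears at zero speed.
; Optional prints show live speed and, once until ResetTimePrint is triggered, the elapsed time and straight-line distance.
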(event Custom|There)

(event Custom|Reset%20New%20Timer
  (Utilities|FlowControl|DoOnce false) ; enters at Reset
)

(event Custom|ResetTimePrint
  (bind _timer (Variables|Default|GetTimer))
  (bind _returnvalue (Class|KismetSystemLibrary|GetTimerElapsedTimeHandle _timer))
  (Utilities|FlowControl|DoOnce false) ; enters at Reset
)

(event EventBeginPlay
  (bind _outactors (Actor|GetAllActorsOfClass "/Game/RollingBP/Blueprints/PhysicsBallBP.PhysicsBallBP_C"))
  (Variables|Default|SetBall (Utilities|Array|Get(acopy) _outactors)))

(event EventTick
  (params (DeltaSeconds :type Float%20%28single-precision%29))
  (bind _ball (Variables|Default|GetBall))
  (bind _ball_2 (Variables|Default|GetBall))
  (bind _returnvalue (Transformation|GetVelocity _ball_2))
  (bind _returnvalue_2 (Math|Vector|VectorLength _returnvalue))
  (if (Variables|Default|GetPrintSpeed?)
    (Development|PrintString (Utilities|String|ToString(Float) _returnvalue_2)))
  (if (== _returnvalue_2 0.0)
    (Utilities|Time|ClearandInvalidateTimerbyHandle (Variables|Default|GetTimer))
    (CallFunction|ResetNewTimer)
    (elif (> _returnvalue_2 0.1)
      (Utilities|FlowControl|Sequence
        (:then_0
          (Utilities|FlowControl|DoOnce false
            (:Completed
              (bind _returnvalue_3 (Utilities|Time|SetTimerbyEvent (delegate Custom|There) 1e+02 true))
              (Variables|Default|SetTimer _returnvalue_3)
              (Variables|Default|SetBallStartLoc (Transformation|GetActorLocation (Variables|Default|GetBall))))))
        (:then_1
          (if (> (Math|Vector|VectorLength (Transformation|GetVelocity _ball)) (Variables|/Game/RollingBP/Blueprints/PhysicsBallBP.PhysicsBallBP_C|GetSpeedLock _ball))
            (Utilities|FlowControl|DoOnce false
              (:Completed
                (if (Variables|Default|GetPrintTimeTilFullSpeedandDistance?)
                  (Development|PrintString (Utilities|String|Append "Time Till Full Speed: " (Utilities|String|ToString(Float) (Class|KismetSystemLibrary|GetTimerElapsedTimeHandle (Variables|Default|GetTimer)))))
                  (Development|PrintString (Utilities|String|Append "Distance Covered Over " (Utilities|String|ToString(Float) (Class|KismetSystemLibrary|GetTimerElapsedTimeHandle (Variables|Default|GetTimer))) "Seconds : " (Utilities|String|ToString(Float) (Math|Vector|VectorLength (- (Variables|Default|GetBallStartLoc) (Transformation|GetActorLocation (Variables|Default|GetBall))))))))))))))))

(fn ConstructionScript)