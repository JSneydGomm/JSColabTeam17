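; Design tool actor that measures and optionally prints how long the PhysicsBallBP ball stays airborne during jumps.
; Each tick it traces down from the first ball found against WorldStatic, treating a gap over a small threshold as airborne.
; Leaving the ground starts a long looping timer once through a DoOnce, used as a stopwatch with an empty event.
; Landing prints the elapsed time when enabled, clears the timer and re-arms the DoOnce.
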(event Custom|HelloThere)

(event Custom|Reset
  (Utilities|FlowControl|DoOnce false) ; enters at Reset
)

(event EventBeginPlay
  (bind _outactors (Actor|GetAllActorsOfClass "/Game/RollingBP/Blueprints/PhysicsBallBP.PhysicsBallBP_C"))
  (Variables|Default|SetBall (Utilities|Array|Get(acopy) _outactors)))

(event EventTick
  (params (DeltaSeconds :type Float%20%28single-precision%29))
  (bind _ball (Variables|Default|GetBall))
  (bind _returnvalue (Transformation|GetActorLocation _ball))
  (bind _outhit (Collision|LineTraceForObjects _returnvalue (+ _returnvalue "0.000000, 0,-1000.000000") (Utilities|Array|MakeArray "ObjectTypeQuery1") false 0 "None"))
  (if (> (Math|Vector|VectorLength (- (.Location (Collision|BreakHitResult _outhit)) (.TraceStart (Collision|BreakHitResult _outhit)))) 6e+01)
    (Utilities|FlowControl|DoOnce false
      (:Completed
        (bind _returnvalue_2 (Utilities|Time|SetTimerbyEvent (delegate Custom|HelloThere) 1e+02 true))
        (Variables|Default|SetJumpTimer _returnvalue_2)))
    (elif (Utilities|Time|IsValidTimerHandle (Variables|Default|GetJumpTimer))
      (if (Variables|Default|GetPrintTimeInAir?)
        (Development|PrintString (Utilities|String|Append "Time In Air: " (Utilities|String|ToString(Float) (Class|KismetSystemLibrary|GetTimerElapsedTimeHandle (Variables|Default|GetJumpTimer))))))
      (Utilities|Time|ClearandInvalidateTimerbyHandle (Variables|Default|GetJumpTimer))
      (CallFunction|Reset))))

(fn ConstructionScript)